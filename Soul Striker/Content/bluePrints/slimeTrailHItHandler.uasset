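; Short-lived slime trail hazard that slows the KnightOfLight while it stands in the trail's box.
; On BeginPlay it starts a fast looping timer, then destroys itself after a fixed delay.
; The timer polls the box's overlapping actors and calls MovementSlow on the first knight found.
; The begin-overlap event is empty, and an older direct walk-speed change is left disconnected.
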(event OnComponentBeginOverlap(Box)
  (params (OverlappedComponent :type Primitive%20Component%20Object%20Reference) (OtherActor :type Actor%20Object%20Reference) (OtherComp :type Primitive%20Component%20Object%20Reference) (OtherBodyIndex :type Integer) (bFromSweep :type Boolean) (SweepResult :type Hit%20Result%20Structure%20%28by%20ref%29)))

(event Custom|checkForKnight
  (Utilities|Time|SetTimerbyFunctionName 0 "slimeContactCheck" 0.1 true))

(event EventBeginPlay
  (CallFunction|CheckforKnight)
  (Utilities|FlowControl|Delay 1e+01)
  (Actor|DestroyActor))

(fn ConstructionScript)

(fn SlimeContactCheck
  (bind _asknight_of_light (Utilities|Casting|CastToKnightOfLight (Utilities|Array|Get(acopy) (Collision|GetOverlappingActors (Variables|Default|GetBox) "/Game/ThirdPersonBP/Blueprints/KnightOfLight.KnightOfLight_C" :!class /Script/Engine.PrimitiveComponent))))
  (Default|MovementSlow _asknight_of_light))