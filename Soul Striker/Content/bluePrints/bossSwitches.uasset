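; Boss switch actor that toggles BallZapper hazards and destroys itself once both the spirit orb and the knight's sword register on it.
; Cube hits from the orb bounce it and swap two indexed zappers' collision and visibility.
; Box overlaps set the orb and sword flags, also saving orb velocity.
; A looping timer polls both flags, then teleports the knight to PrevLoc, restores health, sets orb charge and destroys the switch.
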(event OnComponentBeginOverlap(Box)
  (params (OverlappedComponent :type Primitive%20Component%20Object%20Reference) (OtherActor :type Actor%20Object%20Reference) (OtherComp :type Primitive%20Component%20Object%20Reference) (OtherBodyIndex :type Integer) (bFromSweep :type Boolean) (SweepResult :type Hit%20Result%20Structure%20%28by%20ref%29))
  (bind _asspirit_orb_og (Utilities|Casting|CastTospiritOrbOG OtherActor)
    (:then
      (bind _returnvalue (Physics|GetPhysicsLinearVelocity (Variables|/Game/bluePrints/spiritOrbOG.spiritOrbOG_C|GetSphere _asspirit_orb_og) "None"))
      (Variables|/Game/bluePrints/spiritOrbOG.spiritOrbOG_C|SetOriginal%20Velocity%20X _asspirit_orb_og (.x _returnvalue))
      (Variables|/Game/bluePrints/spiritOrbOG.spiritOrbOG_C|SetOriginal%20Velocity%20Y _asspirit_orb_og (.y _returnvalue))
      (Variables|Default|SetorbHit? true))
    (:CastFailed
      (bind _asknight_of_light (Utilities|Casting|CastToKnightOfLight OtherActor))
      (Variables|Default|SetswordHit? (== (Variables|/Game/ThirdPersonBP/Blueprints/KnightOfLight.KnightOfLight_C|Getsword _asknight_of_light) OtherComp)))))

(event OnComponentHit(Cube)
  (params (HitComponent :type Primitive%20Component%20Object%20Reference) (OtherActor :type Actor%20Object%20Reference) (OtherComp :type Primitive%20Component%20Object%20Reference) (NormalImpulse :type Vector :default "0, 0, 0") (Hit :type Hit%20Result%20Structure%20%28by%20ref%29))
  (bind _asspirit_orb_og (Utilities|Casting|CastTospiritOrbOG OtherActor))
  (Default|BallBounceNon-Destructible _asspirit_orb_og)
  (bind _outactors (Actor|GetAllActorsOfClass "/Game/bluePrints/ballZapper.ballZapper_C"))
  (Collision|SetCollisionEnabled (Variables|/Game/bluePrints/ballZapper.ballZapper_C|GetBox (Utilities|Array|Get(acopy) _outactors (Variables|Default|GetwhichZapperToDisable))) "NoCollision")
  (Rendering|SetVisibility (Variables|/Game/bluePrints/ballZapper.ballZapper_C|GetStaticMesh (Utilities|Array|Get(acopy) _outactors (Variables|Default|GetwhichZapperToDisable))) false false)
  (Rendering|SetVisibility (Variables|/Game/bluePrints/ballZapper.ballZapper_C|GetStaticMesh1 (Utilities|Array|Get(acopy) _outactors (Variables|Default|GetwhichZapperToDisable))) false false)
  (Rendering|SetVisibility (Variables|/Script/Engine.StaticMeshActor|GetStaticMeshComponent (Utilities|Array|Get(acopy) _outactors (Variables|Default|GetwhichZapperToDisable))) false false)
  (Collision|SetCollisionEnabled (Variables|/Game/bluePrints/ballZapper.ballZapper_C|GetBox (Utilities|Array|Get(acopy) _outactors (Variables|Default|GetwhichZapperToEnable))) "QueryOnly")
  (Rendering|SetVisibility (Variables|/Game/bluePrints/ballZapper.ballZapper_C|GetStaticMesh (Utilities|Array|Get(acopy) _outactors (Variables|Default|GetwhichZapperToEnable))) true false)
  (Rendering|SetVisibility (Variables|/Game/bluePrints/ballZapper.ballZapper_C|GetStaticMesh1 (Utilities|Array|Get(acopy) _outactors (Variables|Default|GetwhichZapperToEnable))) true false)
  (Rendering|SetVisibility (Variables|/Script/Engine.StaticMeshActor|GetStaticMeshComponent (Utilities|Array|Get(acopy) _outactors (Variables|Default|GetwhichZapperToEnable))) true false))

(event Custom|checkBoolsForDeath
  (Utilities|Time|SetTimerbyFunctionName 0 "checkBools" 0.1 true))

(event EventBeginPlay
  (CallFunction|CheckBoolsforDeath))

(fn ConstructionScript)

(fn CheckBools
  (bind _outactors (Actor|GetAllActorsOfClass "bossSwitches_C"))
  (Development|PrintString (Utilities|String|ToString(Integer) (Utilities|Array|Length _outactors)))
  (if (Variables|Default|GetorbHit?)
    (if (Variables|Default|GetswordHit?)
      (bind _outactors_2 (Actor|GetAllActorsOfClass "/Game/ThirdPersonBP/Blueprints/KnightOfLight.KnightOfLight_C"))
      (Transformation|SetActorLocation (Utilities|Array|Get(acopy) _outactors_2) (Variables|/Game/ThirdPersonBP/Blueprints/KnightOfLight.KnightOfLight_C|GetprevLoc (Utilities|Array|Get(acopy) _outactors_2)) false true)
      (if (<= (Variables|/Game/ThirdPersonBP/Blueprints/KnightOfLight.KnightOfLight_C|GetCurrentHealth (Utilities|Array|Get(acopy) _outactors_2)) 6.0)
        (Variables|/Game/ThirdPersonBP/Blueprints/KnightOfLight.KnightOfLight_C|SetCurrentHealth (Utilities|Array|Get(acopy) _outactors_2) (+ (Variables|/Game/ThirdPersonBP/Blueprints/KnightOfLight.KnightOfLight_C|GetCurrentHealth (Utilities|Array|Get(acopy) _outactors_2)) 4.0))
        (else
          (Variables|/Game/ThirdPersonBP/Blueprints/KnightOfLight.KnightOfLight_C|SetCurrentHealth (Utilities|Array|Get(acopy) _outactors_2) (Variables|/Game/ThirdPersonBP/Blueprints/KnightOfLight.KnightOfLight_C|GetMaxHealth (Utilities|Array|Get(acopy) _outactors_2)))))
      (Variables|/Game/ThirdPersonBP/Blueprints/KnightOfLight.KnightOfLight_C|SetOrbCurrentPercent (Utilities|Array|Get(acopy) _outactors_2) 3.0)
      (Actor|DestroyActor))))