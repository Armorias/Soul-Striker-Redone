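; Stationary AI turret that shoots at the player and is destroyed when hit by a spirit orb.
; Each Tick checks range and a Visibility trace, then yaws the top toward the player and fires socket-spawned bullets, paced by a Delay.
; A box overlap saves the orb's velocity before impact triggers its bounce.
; A separate shardDrop event, not called here, scatters heart shards and an orb shard.
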(event OnComponentHit(TurretBase)
  (params (HitComponent :type Primitive%20Component%20Object%20Reference) (OtherActor :type Actor%20Object%20Reference) (OtherComp :type Primitive%20Component%20Object%20Reference) (NormalImpulse :type Vector :default "0, 0, 0") (Hit :type Hit%20Result%20Structure%20%28by%20ref%29))
  (bind _asspirit_orb_og (Utilities|Casting|CastTospiritOrbOG OtherActor))
  (Default|BallBounceDestructible _asspirit_orb_og)
  (Actor|DestroyActor))

(event OnComponentBeginOverlap(Box1)
  (params (OverlappedComponent :type Primitive%20Component%20Object%20Reference) (OtherActor :type Actor%20Object%20Reference) (OtherComp :type Primitive%20Component%20Object%20Reference) (OtherBodyIndex :type Integer) (bFromSweep :type Boolean) (SweepResult :type Hit%20Result%20Structure%20%28by%20ref%29))
  (bind _asspirit_orb_og (Utilities|Casting|CastTospiritOrbOG OtherActor))
  (bind _returnvalue (Physics|GetPhysicsLinearVelocity (Variables|/Game/bluePrints/spiritOrbOG.spiritOrbOG_C|GetSphere _asspirit_orb_og) "None"))
  (Variables|/Game/bluePrints/spiritOrbOG.spiritOrbOG_C|SetOriginal%20Velocity%20X _asspirit_orb_og (.x _returnvalue))
  (Variables|/Game/bluePrints/spiritOrbOG.spiritOrbOG_C|SetOriginal%20Velocity%20Y _asspirit_orb_og (.y _returnvalue)))

(event Custom|RotateTurret
  ;[1 1 1] Update Rotation
  (Transformation|SetWorldRotation (Variables|Default|Getturret_top) (Math|Interpolation|RInterpTo (Transformation|GetWorldRotation (Variables|Default|Getturret_top)) (Math|Rotator|MakeRotator 0.0 0.0 (.Yaw (Math|Rotator|BreakRotator (Math|Rotator|FindLookatRotation (Transformation|GetWorldLocation (Variables|Default|Getturret_top)) (Transformation|GetActorLocation (Game|GetPlayerCharacter 0)))))) (Variables|Default|GetDeltaTime) (Variables|Default|GetRotationSpeed)) false false))

(event Custom|UpdateRange
  ;[1 1 1] Update Range
  (if (<= (Transformation|GetDistanceTo (Game|GetPlayerCharacter 0)) (Variables|Default|GetAttackRange))
    (Variables|Default|SetEnemyInRange true)
    (else
      (Variables|Default|SetEnemyInRange false))))

(event Custom|shardDrop
  (bind _self self)
  (bind _self_2 self)
  (bind _turretbase (Variables|Default|GetTurretBase _self))
  (bind _turretbase_2 (Variables|Default|GetTurretBase _self_2))
  (bind _returnvalue (Transformation|GetWorldTransform _turretbase_2))
  (bind _returnvalue_2 (Transformation|GetWorldTransform _turretbase))
  (for _index (range 0 (Math|Random|RandomIntegerinRange 6 15))
    (Game|SpawnActorfromClass "/Game/bluePrints/heartShard.heartShard_C" (Math|Transform|MakeTransform (.location _returnvalue_2) (.rotation _returnvalue_2) "1,1,1") "AdjustIfPossibleButAlwaysSpawn" 0 0)
    (Utilities|FlowControl|Delay 0.05))
  (Game|SpawnActorfromClass "/Game/bluePrints/orbShard.orbShard_C" (Math|Transform|MakeTransform (.location _returnvalue) (.rotation _returnvalue) "1,1,1") "AdjustIfPossibleButAlwaysSpawn" 0 0))

(event Custom|FireTurret
  ;[1 1 1] Fire Projectile
  (Utilities|FlowControl|Delay (Variables|Default|GetFireRate))
  (Game|SpawnActorfromClass "/Game/bluePrints/AI_Turret/AI_TurretBullet.AI_TurretBullet_C" (Transformation|GetSocketTransform (Variables|Default|Getturret_top) "BulletSocket" "RTS_World") "Undefined" 0 0))

(event Custom|CheckforObstacles
  ;[1 1 1] Check for Obstacles in the way to the player
  (bind _returnvalue (Collision|LineTraceByChannel (Transformation|GetWorldLocation (Variables|Default|Getturret_top)) (Transformation|GetActorLocation (Game|GetPlayerCharacter 0)) "TraceTypeQuery1" false 0 "None"))
  (if _returnvalue
    (Variables|Default|SetInSightLine false)
    (else
      (Variables|Default|SetInSightLine true))))

(event EventTick
  (params (DeltaSeconds :type Float%20%28single-precision%29))
  ;[1 1 1] Game Loop
  (Variables|Default|SetDeltaTime DeltaSeconds)
  (CallFunction|UpdateRange)
  (if (Variables|Default|GetEnemyInRange)
    (CallFunction|CheckforObstacles)
    (if (Variables|Default|GetInSightLine)
      (CallFunction|RotateTurret)
      (CallFunction|FireTurret))))

(fn ConstructionScript)