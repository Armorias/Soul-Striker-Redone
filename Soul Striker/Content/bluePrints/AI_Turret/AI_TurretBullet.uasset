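; AI turret bullet that damages the KnightOfLight player character or registers a shield block.
; A Box overlap checks the component hit: the Shield updates the block meter and leaves the bullet alive, while any other part loses health, refreshes it and destroys the bullet.
; A second sequence branch destroys the bullet when the sweep's hit actor is a superWallTop.
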(event OnComponentBeginOverlap(Box)
  (params (OverlappedComponent :type Primitive%20Component%20Object%20Reference) (OtherActor :type Actor%20Object%20Reference) (OtherComp :type Primitive%20Component%20Object%20Reference) (OtherBodyIndex :type Integer) (bFromSweep :type Boolean) (SweepResult :type Hit%20Result%20Structure%20%28by%20ref%29))
  ;[1 1 1] hit Code
  (Utilities|FlowControl|Sequence
    (:then_0
      (bind _asknight_of_light (Utilities|Casting|CastToKnightOfLight OtherActor))
      ;;[1 1 1] Make sure that the part of the knight hit isn't the shield
      (if (== (Variables|/Game/ThirdPersonBP/Blueprints/KnightOfLight.KnightOfLight_C|Getshield _asknight_of_light) OtherComp)
        (Default|UpdateBlockMeter _asknight_of_light true)
        (else
          ;;[1 1 1] If it isn't, then deal damage to the knight hit.
          (Variables|/Game/ThirdPersonBP/Blueprints/KnightOfLight.KnightOfLight_C|SetCurrentHealth _asknight_of_light (- (Variables|/Game/ThirdPersonBP/Blueprints/KnightOfLight.KnightOfLight_C|GetCurrentHealth _asknight_of_light) 1.0))
          (Default|UpdateHealth _asknight_of_light)
          (Actor|DestroyActor))))
    (:then_1
      ;;[1 1 1] Comment
      (Utilities|Casting|CastTosuperWallTop (.HitActor (Collision|BreakHitResult SweepResult)))
      (Actor|DestroyActor))))

(fn ConstructionScript)